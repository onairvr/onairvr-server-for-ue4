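; Sample player Blueprint that represents tracked left and right hand controllers and gives visual feedback on trigger input.
; On BeginPlay it enables input on its player controller.
; Each tick it shows a controller only while that hand's tracker is available and player 0 is activated.
; Left and right trigger input actions swap the matching controller's material between normal and triggered.
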(event EventTick
  (params (DeltaSeconds :type Float%20%28single-precision%29))
  (bind _returnvalue (Class|AirVRServerFunctionLibrary|IsPlayerActivated))
  ;[1 1 1] Show/Hide Controllers
  (Utilities|FlowControl|Sequence
    (:then_0
      (bind _returnvalue_2 (Class|AirVRServerFunctionLibrary|IsInputDeviceAvailable 0 "LeftHandTracker"))
      (Rendering|SetVisibility (Variables|Default|GetLeftController) (and _returnvalue_2 _returnvalue) false))
    (:then_1
      (bind _returnvalue_3 (Class|AirVRServerFunctionLibrary|IsInputDeviceAvailable 0 "RightHandTracker"))
      (Rendering|SetVisibility (Variables|Default|GetRightController) (and _returnvalue_3 _returnvalue) false))))

(event EventBeginPlay
  ;[1 1 1] Enable Player Input
  (bind _asplayer_controller (Utilities|Casting|CastToPlayerController (Pawn|GetController)))
  (Input|EnableInput _asplayer_controller 0))

(event Input|ActionEvents|InputActionLeftTrigger
  (params (Key :type Key%20Structure :default "None"))
  (bind _leftcontroller (Variables|Default|GetLeftController))
  ;[1 1 1] Process Player Input
  (:Pressed
    (Rendering|Material|SetMaterial _leftcontroller 0 "/Game/Materials/M_Triggered.M_Triggered"))
  (:Released
    (Rendering|Material|SetMaterial _leftcontroller 0 "/Game/Materials/M_Player.M_Player")))

(event Input|ActionEvents|InputActionRightTrigger
  (params (Key :type Key%20Structure :default "None"))
  (bind _rightcontroller (Variables|Default|GetRightController))
  ;[1 1 1] Process Player Input
  (:Pressed
    (Rendering|Material|SetMaterial _rightcontroller 0 "/Game/Materials/M_Triggered.M_Triggered"))
  (:Released
    (Rendering|Material|SetMaterial _rightcontroller 0 "/Game/Materials/M_Player.M_Player")))

(fn ConstructionScript)