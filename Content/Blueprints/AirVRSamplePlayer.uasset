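; AirVRSamplePlayer is the player pawn for an AirVR sample, with camera-relative movement, motion controllers and can throwing.
; Each tick it turns the head mesh to the camera rotation, moves along the camera-rotated input and assigns the player controller ID to both motion controllers.
; The Throw input spawns a short-lived can at the right controller, or a fallback throw point when untracked, launching it with impulse and spin.
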(event EventTick
  (params (DeltaSeconds :type Float%20%28single-precision%29))
  ;[1 1 1] Update The Rotation of Head Mesh
  (bind _returnvalue (|GetCameraRotationOfPlayerController))
  (Transformation|SetWorldRotation (Variables|Default|GetHeadLocator) _returnvalue false false)
  ;[1 1 1] Move Player
  (bind _asplayer_controller (Utilities|Casting|CastToPlayerController (Pawn|GetController)))
  (Pawn|Input|AddMovementInput (Math|Vector|RotateVector (* (Math|Vector|MakeVector (.Y (Math|Vector2D|BreakVector2D (Class|AirVRSampleHelperFunctionLibrary|GetPlayerMoveInputDirection _asplayer_controller))) (.X (Math|Vector2D|BreakVector2D (Class|AirVRSampleHelperFunctionLibrary|GetPlayerMoveInputDirection _asplayer_controller))) 0.0) (Variables|Default|GetSpeed)) (Camera|GetCameraRotation (Variables|/Script/Engine.PlayerController|GetPlayerCameraManager _asplayer_controller))) 1.0 false)
  ;[1 1 1] Motion Controller Setting
  (bind _returnvalue_2 (Class|GameplayStatics|GetPlayerControllerID _asplayer_controller))
  (bind _output_get (Variables|/Script/HeadMountedDisplay.MotionControllerComponent|SetPlayerIndex (Variables|Default|GetRightController) _returnvalue_2))
  (Variables|/Script/HeadMountedDisplay.MotionControllerComponent|SetPlayerIndex (Variables|Default|GetLeftController) _output_get))

(event EventBeginPlay
  ;[1 1 1] Enable Player Input
  (bind _asplayer_controller (Utilities|Casting|CastToPlayerController (Pawn|GetController)))
  (Input|EnableInput _asplayer_controller 0))

(event Input|ActionEvents|InputActionThrow
  (params (Key :type Key%20Structure))
  (bind _throwcanpoint (Variables|Default|GetThrowCanPoint))
  (bind _rightcontroller (Variables|Default|GetRightController))
  (bind _returnvalue (Class|MotionControllerComponent|IsTracked _rightcontroller))
  (bind _returnvalue_2 (select _returnvalue _rightcontroller _throwcanpoint))
  (bind _returnvalue_3 (Transformation|GetWorldRotation _returnvalue_2))
  ;[1 1 1] Throw
  (:Pressed
    (bind _returnvalue_4 (Game|SpawnActorfromClass (Variables|Default|GetCanClass) (Math|Transform|MakeTransform (Transformation|GetWorldLocation _returnvalue_2) _returnvalue_3) "Undefined" 0 0))
    (Physics|AddImpulse (Variables|/Game/Blueprints/Can.Can_C|GetCan _returnvalue_4) (Math|Vector|RotateVector "90.000000, 0, 0" _returnvalue_3) "None" false)
    (Class|PrimitiveComponent|AddTorqueinRadians (Variables|/Game/Blueprints/Can.Can_C|GetCan _returnvalue_4) (Math|Vector|RotateVector "0,250.000000, 0" _returnvalue_3) "None" false)
    (Actor|SetLifeSpan _returnvalue_4 8.0)))

(fn ConstructionScript)